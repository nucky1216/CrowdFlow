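; Test agent actor for flow-field movement and neighbour repulsion, registered as a Mass entity in FlowFieldNeiboursSubsystem on construction and labelled with its EntityID.
; DeltaMove gets the next location from FlowFieldVoxelBuilder, moves without sweep and draws repel, guidance, plane and final force arrows.
; Tick leaves DeltaMove unwired, and BeginPlay only randomises MaxSpeed and binds the registration event.
; Other functions debug navmesh paths, neighbours and the subsystem map.
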(event EventBeginPlay
  (EventDispatchers|BindEventtoOnEntityRegistered (Subsystems|GetFlowFieldNeiboursSubsystem) (EventDispatchers|CreateEvent :!event DeltaMove))
  (Variables|Default|SetMaxSpeed (Math|Random|RandomFloatinRange 95.0 1.5e+02)))

(event Collision|EventActorBeginOverlap
  (params (OtherActor :type Actor%20Object%20Reference)))

(event EventTick
  (params (DeltaSeconds :type Float%20%28single-precision%29)))

(fn ConstructionScript
  (CallFunction|InitalMove))

(fn ShowSampledFlow
  (params (Duration :type Float%20%28single-precision%29))
  (bind _returnvalue (Transformation|GetActorLocation))
  (bind _offset (LocalVariables|GetOffset))
  (bind _returnvalue_2 (+ _returnvalue _offset))
  (Utilities|FlowControl|Sequence
    (:then_1
      (bind (_repelforce _guidanceforce _planeforce _returnvalue_3) (Class|FlowFieldVoxelBuilder|GetFlowbyPoly (Variables|Default|GetFlowFieldVoxelBuilder) (Transformation|GetActorLocation) (Variables|Default|GetVelocity) "50.000000,50.000000,50.000000"))
      (LocalVariables|SetRepelForce _repelforce)
      (LocalVariables|SetGuidanceForce _guidanceforce)
      (LocalVariables|SetPlaneForce _planeforce)
      (LocalVariables|SetFinalForce _returnvalue_3)
      (Rendering|Debug|DrawDebugArrow _returnvalue_2 (+ _returnvalue_2 (* (Variables|Default|GetSampleStep) (LocalVariables|GetFinalForce))) 1e+02 "(R=0.408038,G=1.000000,B=0.000000,A=1.000000)" Duration 1e+01)
      (Rendering|Debug|DrawDebugArrow _returnvalue_2 (+ _returnvalue_2 (* (LocalVariables|GetRepelForce) (Variables|Default|GetSampleStep))) 1e+02 "(R=1.000000,G=0.057486,B=0.000000,A=1.000000)" Duration 1e+01)
      (Rendering|Debug|DrawDebugArrow _returnvalue_2 (+ _returnvalue_2 (* (LocalVariables|GetGuidanceForce) (Variables|Default|GetSampleStep))) 1e+02 "(R=0.211700,G=0.083511,B=1.000000,A=1.000000)" Duration 1e+01)
      (Rendering|Debug|DrawDebugArrow _returnvalue_2 (+ _returnvalue_2 (* (LocalVariables|GetPlaneForce) (Variables|Default|GetSampleStep))) 1e+02 "(R=0.897140,G=1.000000,B=0.884286,A=1.000000)" Duration 1e+01))))

(fn FindPath
  (bind _returnvalue (Class|NavigationSystemV1|FindPathtoLocationSynchronously (Class|NavigationSystemV1|GetNavigationSystem) (Transformation|GetActorLocation) (Variables|Default|GetPath%20End) 0 0))
  (LocalVariables|SetPathPoints (Variables|/Script/NavigationSystem.NavigationPath|GetPathPoints _returnvalue))
  (for _index (range 1 (- (Utilities|Array|Length (Variables|/Script/NavigationSystem.NavigationPath|GetPathPoints _returnvalue)) 1))
    (Rendering|Debug|DrawDebugArrow (Utilities|Array|Get(acopy) (LocalVariables|GetPathPoints) (- _index 1)) (Utilities|Array|Get(acopy) (LocalVariables|GetPathPoints) _index) 5e+01 "(R=0.000000,G=0.226994,B=1.000000,A=1.000000)" 5.0 5.0)))

(fn ShowFlow
  (CallFunction|ShowSampledFlow 5.0))

(fn GetNeibours
  (Class|FlowFieldVoxelBuilder|DebugDrawNeibours (Variables|Default|GetFlowFieldVoxelBuilder) self 10))

(fn Registry
  (Class|FlowFieldNeiboursSubsystem|RegistryMassEntity (Subsystems|GetFlowFieldNeiboursSubsystem) self))

(fn DebugOutput
  (Class|FlowFieldNeiboursSubsystem|DebugMap (Subsystems|GetFlowFieldNeiboursSubsystem)))

(fn ResetMap
  (Class|FlowFieldNeiboursSubsystem|ResetMap (Subsystems|GetFlowFieldNeiboursSubsystem)))

(fn InitialSubsystem
  (Class|FlowFieldNeiboursSubsystem|InitializeManual (Subsystems|GetFlowFieldNeiboursSubsystem)))

(fn NeibourRepel
  (Class|FlowFieldVoxelBuilder|GetForcefromNeibours (Variables|Default|GetFlowFieldVoxelBuilder) self))

(fn DeltaMove
  (params (A :type Float%20%28double-precision%29))
  (bind _returnvalue (Class|FlowFieldVoxelBuilder|DeltaMove (Variables|Default|GetFlowFieldVoxelBuilder) self (Variables|Default|GetVelocity) (Variables|Default|GetMaxSpeed) (Variables|Default|GetMass)))
  (Transformation|SetActorLocation _returnvalue false false)
  (CallFunction|ShowSampledFlow (+ A 0.001)))

(fn InitalMove
  (CallFunction|Registry)
  (Rendering|Components|TextRender|SetText (Variables|Default|GetTextRender) (Utilities|Text|ToText(String) (Variables|Default|GetEntityID))))