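; Test-map spawner that populates a flow field with BP_Move agents for movement.
; Spawn first destroys all existing BP_Move actors, then loops up to Num, cycling through the FlowField's polygons and picking a random reachable navigation point near each center.
; Each spawned agent receives its index as EntityID and a reference to the flow field builder, then runs InitalMove.
; The event graph is empty, so Spawn is not triggered from within this Blueprint.
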(event EventBeginPlay)

(event Collision|EventActorBeginOverlap
  (params (OtherActor :type Actor%20Object%20Reference)))

(event EventTick
  (params (DeltaSeconds :type Float%20%28single-precision%29)))

(fn ConstructionScript)

(fn Spawn
  (CallFunction|ClearMove)
  (LocalVariables|SetPolyNum (Utilities|Array|Length (Class|FlowFieldVoxelBuilder|GetFlowPoly (Variables|Default|GetFlowField))))
  (for _index (range 1 (Variables|Default|GetNum))
    (if (.ReturnValue (AI|Navigation|GetRandomReachablePointinRadius (.Center (Utilities|Struct|BreakNavPolyFlow (Utilities|Array|Get(acopy) (Class|FlowFieldVoxelBuilder|GetFlowPoly (Variables|Default|GetFlowField)) (Math|Integer|%(Integer) (* _index 1) (LocalVariables|GetPolyNum))))) 5e+02 0 0))
      (bind _returnvalue (Game|SpawnActorfromClass "/CrowdFlow/TestMaps/BP_Move.BP_Move_C" (Math|Conversions|ToTransform(Vector) (.RandomLocation (AI|Navigation|GetRandomReachablePointinRadius (.Center (Utilities|Struct|BreakNavPolyFlow (Utilities|Array|Get(acopy) (Class|FlowFieldVoxelBuilder|GetFlowPoly (Variables|Default|GetFlowField)) (Math|Integer|%(Integer) (* _index 1) (LocalVariables|GetPolyNum))))) 5e+02 0 0))) "Undefined" "MultiplyWithRoot" 0 0))
      (Variables|/Script/CrowdFlow.EntityActor|SetEntityID _returnvalue (Class|KismetMathLibrary|ToInt64(Integer) _index))
      (Variables|/Script/CrowdFlow.EntityActor|SetFlowFieldVoxelBuilder _returnvalue (Variables|Default|GetFlowField))
      (Default|InitalMove _returnvalue))))

(fn ClearMove
  (bind _outactors (Actor|GetAllActorsOfClass "/CrowdFlow/TestMaps/BP_Move.BP_Move_C"))
  (for _array_element _outactors
    (Actor|DestroyActor _array_element)))