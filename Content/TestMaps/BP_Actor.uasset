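; Test actor for inspecting and visualizing a flow field, with no active event logic.
; Test averages flow directions from grid cells at Offsets around the actor, weighted by inverse distance between each direction vector and the actor's location, with optional debug arrows.
; ShowGridHeat clears and respawns colored BP_Arrow actors for each flow polygon's direction, normal and boundary-edge normals.
; FindPath draws a synchronous navigation path to PathEnd for debugging.
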(event EventBeginPlay)

(event Collision|EventActorBeginOverlap
  (params (OtherActor :type Actor%20Object%20Reference)))

(fn ConstructionScript)

(fn Test
  (for _array_element (LocalVariables|GetOffsets)
    (bind (_1_dist _flow_direction) (CallFunction|DrawLine _array_element))
    (LocalVariables|SetTotalWeight (+ (LocalVariables|GetTotalWeight) _1_dist))
    (LocalVariables|SetTotalDir (+ _flow_direction (LocalVariables|GetTotalDir))))
  (return (/ (LocalVariables|GetTotalDir) (LocalVariables|GetTotalWeight))))

(fn DrawLine
  (params (Offset :type Int%20Vector%20Structure) (LineColor :type Linear%20Color%20Structure))
  (bind _returnvalue (Transformation|GetActorLocation))
  (bind _flowfield (Variables|Default|GetFlowField))
  (bind _returnvalue_2 (Class|FlowFieldVoxelBuilder|GetGridIndex _flowfield _returnvalue))
  (bind _flowfield_2 (Variables|/Script/CrowdFlow.FlowFieldVoxelBuilder|GetFlowField _flowfield))
  (bind _a2 (Utilities|+ Offset _returnvalue_2))
  (bind _value (Utilities|Map|Find _flowfield_2 _a2))
  (bind (_worldposition _flowdirection _heat _flag _bisvalid) (Utilities|Struct|BreakFlowVoxel _value))
  (bind _returnvalue_3 (Math|Vector|Distance(Vector) _flowdirection _returnvalue))
  (bind _returnvalue_4 (Math|Float|SafeDivide 1.0 _returnvalue_3))
  (if _bisvalid
    (Utilities|FlowControl|Sequence
      (:then_0
        (if (Variables|Default|GetDebug)
          (Rendering|Debug|DrawDebugArrow _returnvalue (+ _returnvalue (* _flowdirection 2e+02)) 5e+01 LineColor 5.0 1e+01)
          (Class|DimensioBPLibrary|PrintLog (Utilities|String|ToString(Integer) _a2))))
      (:then_1
        (return _returnvalue_4 (* _returnvalue_4 _flowdirection))))))

(fn FindPath
  (bind _returnvalue (Class|NavigationSystemV1|FindPathtoLocationSynchronously (Class|NavigationSystemV1|GetNavigationSystem) (Transformation|GetActorLocation) (Variables|Default|GetPath%20End) 0 0))
  (LocalVariables|SetPathPoints (Variables|/Script/NavigationSystem.NavigationPath|GetPathPoints _returnvalue))
  (for _index (range 1 (- (Utilities|Array|Length (Variables|/Script/NavigationSystem.NavigationPath|GetPathPoints _returnvalue)) 1))
    (Rendering|Debug|DrawDebugArrow (Utilities|Array|Get(acopy) (LocalVariables|GetPathPoints) (- _index 1)) (Utilities|Array|Get(acopy) (LocalVariables|GetPathPoints) _index) 5e+01 "(R=0.000000,G=0.226994,B=1.000000,A=1.000000)" 5.0 5.0)))

(fn ShowGridHeat
  (Utilities|FlowControl|Sequence
    (:then_0
      (CallFunction|ClearArrows))
    (:then_2
      (for (_array_element _array_index) (Class|FlowFieldVoxelBuilder|GetFlowPoly (Variables|Default|GetFlowField))
        (LocalVariables|SetVerts (.PolyVerts (Utilities|Struct|BreakNavPolyFlow _array_element)))
        (LocalVariables|SetBEdges (.BoundaryEdge (Utilities|Struct|BreakNavPolyFlow _array_element)))
        (LocalVariables|SetEdgeNormals (.BoundaryEdgeNormal (Utilities|Struct|BreakNavPolyFlow _array_element)))
        (Utilities|FlowControl|Sequence
          (:then_0
            (bind _returnvalue (Game|SpawnActorfromClass "/CrowdFlow/TestMaps/BP_Arrow.BP_Arrow_C" (Math|Transform|MakeTransform (.Center (Utilities|Struct|BreakNavPolyFlow _array_element)) (Math|Rotator|MakeRotfromX (.FlowDirection (Utilities|Struct|BreakNavPolyFlow _array_element)))) "Undefined" "MultiplyWithRoot" 0 0))
            (Utilities|Array|Add (Variables|Default|GetArrow) _returnvalue)
            (Default|SetColor _returnvalue "(R=0.018901,G=1.000000,B=0.000000,A=1.000000)"))
          (:then_1
            (for (_array_element_2 _array_index_2) (LocalVariables|GetBEdges)
              (bind _returnvalue_2 (Game|SpawnActorfromClass "/CrowdFlow/TestMaps/BP_Arrow.BP_Arrow_C" (Math|Transform|MakeTransform (/ (+ (Utilities|Array|Get(acopy) (LocalVariables|GetVerts) _array_element_2) (Utilities|Array|Get(acopy) (LocalVariables|GetVerts) (Math|Integer|%(Integer) (+ _array_element_2 1) (Utilities|Array|Length (LocalVariables|GetVerts))))) 2.0) (Math|Rotator|MakeRotfromX (Utilities|Array|Get(acopy) (LocalVariables|GetEdgeNormals) _array_index_2))) "Undefined" "MultiplyWithRoot" 0 0))
              (Utilities|Array|Add (Variables|Default|GetArrow) _returnvalue_2)
              (Default|SetColor _returnvalue_2 "(R=1.000000,G=0.842913,B=0.000000,A=1.000000)")))
          (:then_2
            (bind _returnvalue_3 (Game|SpawnActorfromClass "/CrowdFlow/TestMaps/BP_Arrow.BP_Arrow_C" (Math|Transform|MakeTransform (.Center (Utilities|Struct|BreakNavPolyFlow _array_element)) (Math|Rotator|MakeRotfromX (.PolyNormal (Utilities|Struct|BreakNavPolyFlow _array_element)))) "Undefined" "MultiplyWithRoot" 0 0))
            (Default|SetColor _returnvalue_3 "(R=0.961578,G=1.000000,B=0.899221,A=1.000000)")))))))

(fn ClearArrows
  (Utilities|FlowControl|Sequence
    (:then_0
      (for _array_element (Variables|Default|GetArrow)
        (Utilities|IsValid _array_element
          (:Is%20Valid
            (Actor|DestroyActor _array_element))))
      (Utilities|Array|Clear (Variables|Default|GetArrow)))
    (:then_1
      (bind _outactors (Actor|GetAllActorsOfClass "/CrowdFlow/TestMaps/BP_Arrow.BP_Arrow_C"))
      (for _array_element_2 _outactors
        (Utilities|IsValid _array_element_2
          (:Is%20Valid
            (Actor|DestroyActor _array_element_2)))))))